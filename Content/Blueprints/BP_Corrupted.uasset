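; BP_Corrupted is a shop visitor that randomly either steals an item or visits the shopkeeper.
; On BeginPlay it picks a random BPI_Stealable actor or walks to the Shop trigger volume.
; Theft moves near the target, retrying on failure, attaches it to the hand socket and heads for the Exit volume.
; Shop interactions notify BP_Shopkeep, report the requested furniture as non-thieving on Update, then leave the same way.
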(event EventBeginPlay
  (bind _returnvalue (Math|Random|RandomBool))
  (|CallParentFunction)
  ;[0.15 0.15 0.15 0.5] Steal
  (if (not (Class|KismetMathLibrary|XORBoolean _returnvalue (Variables|Default|GetPreviousAction)))
    (Variables|Default|SetPreviousAction _returnvalue)
    (bind _outactors (Actor|GetAllActorswithInterface "/Game/Blueprints/BPI_Stealable.BPI_Stealable_C"))
    (bind _asbpi_stealable (Utilities|Casting|CastToBPI_Stealable (.OutItem (Utilities|Array|Random _outactors))))
    (CallFunction|Steal _asbpi_stealable)
    (else
      (Variables|Default|SetPreviousAction _returnvalue)
      (bind _outactors_2 (Actor|GetAllActorsOfClasswithTag "/Script/Engine.TriggerVolume" "Shop"))
      (AI|AIMoveTo self "0, 0, 0" (Utilities|Array|Get(acopy) _outactors_2) 5.0 false))))

(event Collision|EventActorBeginOverlap
  (params (OtherActor :type Actor%20Object%20Reference)))

(event EventTick
  (params (DeltaSeconds :type Float%20%28single-precision%29)))

(event EventEndInteraction
  (params (Sender :type BPI%20Interaction%20Interface))
  ;[0.15 0.15 0.15 0.5 36] Interactions
  (bind _outactors (Actor|GetAllActorsOfClasswithTag "/Script/Engine.TriggerVolume" "Exit"))
  (AI|AIMoveTo self "0, 0, 0" (Utilities|Array|Get(acopy) _outactors) 5.0 false))

(event EventBeginInteraction
  (params (Sender :type BPI%20Interaction%20Interface) (InteractionMetadata :type S%20Interaction%20Metadata%20Structure))
  ;[0.15 0.15 0.15 0.5 36] Interactions
  (Audio|Components|Audio|Play (Variables|Default|GetSpeak) 0.0)
  (bind _returnvalue (Actor|GetActorOfClass "/Game/Blueprints/BP_Shopkeep.BP_Shopkeep_C"))
  (Default|BeginInteraction _returnvalue self))

(event EventUpdate
  (params (Sender :type BPI%20Interaction%20Interface) (InteractionMetadata :type S%20Interaction%20Metadata%20Structure))
  ;[0.15 0.15 0.15 0.5 36] Interactions
  (Default|ReceiveUpdate Sender self (Utilities|Struct|MakeS_InteractionMetadata true (Variables|Default|GetRequestedFurniture) false))
  (CallFunction|EndInteraction))

(event EventBeginPurchase
  (params (Purchase :type S%20Purchase%20Structure))
  ;[0.15 0.15 0.15 0.5 36] Interactions
)

(event EventEndPurchase
  (params (Purchase :type S%20Purchase%20Structure))
  ;[0.15 0.15 0.15 0.5 36] Interactions
)

(event EventSteal
  (params (Target :type BPI%20Stealable%20Interface))
  ;[0.15 0.15 0.15 0.5 36] Interactions
  (bind _asactor (Utilities|Casting|CastToActor Target))
  (bind _randomlocation (Class|NavigationSystemV1|GetRandomLocationinNavigableRadius (Transformation|GetActorLocation _asactor) 2.5e+02 0 0))
  (AI|AIMoveTo self _randomlocation 0 1e+02 true
    (:OnSuccess
      (Collision|SetActorEnableCollision _asactor false)
      (Transformation|AttachActorToActor _asactor self "hand" "SnapToTarget" "SnapToTarget" "SnapToTarget" true)
      (CallFunction|EndInteraction))
    (:OnFail
      (Utilities|FlowControl|Delay 2.0)
      (CallFunction|Steal Target))))

(fn ConstructionScript)