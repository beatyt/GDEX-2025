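; Player character Blueprint that provides camera control and acts as the player's side of customer interactions and furniture orders.
; Enhanced Input pans and rotates through controller yaw and pitch and zooms by clamping spring arm length, while WASD movement is left unimplemented.
; Interaction events track an ActiveCustomer and reply through ReceiveUpdate when interactions begin or orders are placed or fulfilled, clearing it when interaction or purchase ends.
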(event Custom|OrderPlaced
  (params (DesiredClass :type BP%20Furniture%20Base%20Class%20Reference) (CustomerRequesting :type BPI%20Interaction%20Interface))
  (Variables|Default|SetActiveCustomer CustomerRequesting)
  (Default|ReceiveUpdate CustomerRequesting self))

(event Custom|OrderFulfiled
  (params (CustomerRequesting :type BPI%20Interaction%20Interface) (Desired%20Class :type BP%20Furniture%20Base%20Class%20Reference) (Furniture :type BP%20Furniture%20Base%20Object%20Reference))
  (Default|ReceiveUpdate (Variables|Default|GetActiveCustomer) self (Utilities|Struct|MakeS_InteractionMetadata false "(FurnitureName_2_8EFB08124DDC437CD39BBFA784EA4141=\"\",FurnitureCost_5_A532AD904FCD1F791C40BD9367D6E619=0.000000,FurnitureMesh_8_E86097404701EDAFE42A5B985457B673=None,FurnitureBlueprint_11_CE3092FE4FF4BAEF0473709F8125EE1D=None,FurnitureProfit_14_1DC34B26450ED0C95E290284BFFC06B8=0.000000)" false true true))
  (Development|PrintString "Order Done"))

(event Input|EnhancedActionEvents|EnhancedInputActionIA_RotateCamera
  (params (ActionValue :type Vector%202D%20Structure) (ElapsedSeconds :type Float%20%28double-precision%29) (TriggeredSeconds :type Float%20%28double-precision%29) (InputAction :type Input%20Action%20Object%20Reference :default "/Game/Blueprints/GameLogic/Controls/IA_RotateCamera.IA_RotateCamera"))
  (bind (_x _y) (Math|Vector2D|BreakVector2D ActionValue))
  (Pawn|Input|AddControllerYawInput _x)
  (Pawn|Input|AddControllerPitchInput _y))

(event Input|EnhancedActionEvents|EnhancedInputActionIA_CameraPan
  (params (ActionValue :type Vector%202D%20Structure) (ElapsedSeconds :type Float%20%28double-precision%29) (TriggeredSeconds :type Float%20%28double-precision%29) (InputAction :type Input%20Action%20Object%20Reference :default "/Game/Blueprints/GameLogic/Controls/IA_CameraPan.IA_CameraPan"))
  (Pawn|Input|AddControllerYawInput (.x ActionValue))
  (Pawn|Input|AddControllerPitchInput (.y ActionValue)))

(event Input|EnhancedActionEvents|EnhancedInputActionIA_CameraZoom
  (params (ActionValue :type Float%20%28double-precision%29) (ElapsedSeconds :type Float%20%28double-precision%29) (TriggeredSeconds :type Float%20%28double-precision%29) (InputAction :type Input%20Action%20Object%20Reference :default "/Game/Blueprints/GameLogic/Controls/IA_CameraZoom.IA_CameraZoom"))
  (bind _springarm (Variables|Default|GetSpringArm))
  (Variables|/Script/Engine.SpringArmComponent|SetTargetArmLength _springarm (Math|Float|Clamp(Float) (+ (Variables|/Script/Engine.SpringArmComponent|GetTargetArmLength _springarm) (* ActionValue (Variables|Default|GetZoomSpeed))) 1e+02 1e+03)))

(event Input|EnhancedActionEvents|EnhancedInputActionIA_ForwardBack
  (params (ActionValue :type Vector%202D%20Structure) (ElapsedSeconds :type Float%20%28double-precision%29) (TriggeredSeconds :type Float%20%28double-precision%29) (InputAction :type Input%20Action%20Object%20Reference :default "/Game/Blueprints/GameLogic/Controls/IA_ForwardBack.IA_ForwardBack"))
  ;[0.15 0.15 0.15 0.5] Currently  moves the camerea on wasd according to rotation, but we rotate around the spring arm not the spring arm itself. If we want to implement WASD, need to adjust roation logic for this.
)

(event Input|EnhancedActionEvents|EnhancedInputActionIA_LeftRight
  (params (ActionValue :type Vector%202D%20Structure) (ElapsedSeconds :type Float%20%28double-precision%29) (TriggeredSeconds :type Float%20%28double-precision%29) (InputAction :type Input%20Action%20Object%20Reference :default "/Game/Blueprints/GameLogic/Controls/IA_LeftRight.IA_LeftRight"))
  ;[0.15 0.15 0.15 0.5] Currently  moves the camerea on wasd according to rotation, but we rotate around the spring arm not the spring arm itself. If we want to implement WASD, need to adjust roation logic for this.
)

(event EventBeginPlay)

(event Collision|EventActorBeginOverlap
  (params (OtherActor :type Actor%20Object%20Reference)))

(event EventTick
  (params (DeltaSeconds :type Float%20%28single-precision%29)))

(event EventBeginInteraction
  (params (Sender :type BPI%20Interaction%20Interface) (InteractionMetadata :type S%20Interaction%20Metadata%20Structure))
  ;[0.15 0.15 0.15 0.5 36] Interactions
  (Variables|Default|SetActiveCustomer Sender)
  (bind _asbpi_interaction (Utilities|Casting|CastToBPI_Interaction Sender))
  (Default|ReceiveUpdate _asbpi_interaction self))

(event EventEndInteraction
  (params (Sender :type BPI%20Interaction%20Interface))
  ;[0.15 0.15 0.15 0.5 36] Interactions
  ;;[0.15 0.15 0.15 0.5] Do nothing
  (Variables|Default|SetActiveCustomer 0))

(event EventUpdate
  (params (Sender :type BPI%20Interaction%20Interface) (InteractionMetadata :type S%20Interaction%20Metadata%20Structure))
  ;[0.15 0.15 0.15 0.5 36] Interactions
  (if (.EndInteraction? (Utilities|Struct|BreakS_InteractionMetadata InteractionMetadata))
    (CallFunction|EndInteraction)))

(event EventBeginPurchase
  (params (Purchase :type S%20Purchase%20Structure) (RequestingCustomer :type BPI%20Interaction%20Interface))
  ;[0.15 0.15 0.15 0.5 36] Interactions
)

(event EventEndPurchase
  (params (Purchase :type S%20Purchase%20Structure))
  ;[0.15 0.15 0.15 0.5 36] Interactions
  (Variables|Default|SetActiveCustomer 0))

(fn ConstructionScript)