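; Dungeon game mode that spawns randomly chosen customer NPCs at the entrance on a repeating timer.
; BeginPlay caches tagged TargetPoints for entrance, counter and workbench, shows the cursor, and sets the random-interval timer inside that loop.
; Each spawned class leaves the available pool until the following spawn, preventing back-to-back repeats.
; Setup has each customer choose a requested item and speak; the AI move to the counter is disconnected.
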(event Custom|SpawnNewCustomer
  ;[0.15 0.15 0.15 0.5 36] Spawning
  (bind _output_get (Variables|Default|SetCurrentSpawn (.OutItem (Utilities|Array|Random (Variables|Default|GetAvailableCustomers)))))
  (bind _returnvalue (Game|SpawnActorfromClass _output_get (Transformation|GetActorTransform (Variables|Default|GetNPCEntranceRef)) "Undefined" "MultiplyWithRoot" 0 0))
  (if (Utilities|IsValidClass (Variables|Default|GetPreviousSpawn))
    (Utilities|Array|Add (Variables|Default|GetAvailableCustomers) (Variables|Default|GetPreviousSpawn))
    (Variables|Default|SetPreviousSpawn (Variables|Default|GetCurrentSpawn))
    (Utilities|Array|RemoveItem (Variables|Default|GetAvailableCustomers) (Variables|Default|GetCurrentSpawn))
    (CallFunction|Setup _returnvalue)
    (else
      (Utilities|Array|RemoveItem (Variables|Default|GetAvailableCustomers) (Variables|Default|GetCurrentSpawn))
      (Variables|Default|SetPreviousSpawn (Variables|Default|GetCurrentSpawn))
      (CallFunction|Setup _returnvalue))))

(event Custom|Setup
  (params (CurrentCustomer :type BP%20Customer%20Base%20Object%20Reference))
  ;[0.15 0.15 0.15 0.5 36] Spawning
  ;;[0.15 0.15 0.15 0.5 36] Could probably move these onto the BP Customer Base in BeginPlay or an Init
  (bind _output_get (Variables|Default|SetCurrentCustomer CurrentCustomer))
  (Default|SetRequestedItem (Variables|Default|GetCurrentCustomer))
  (Default|SaySomethingFunny (Variables|Default|GetCurrentCustomer)))

(event EventBeginPlay
  (bind _outactors (Actor|GetAllActorsOfClass "/Script/Engine.TargetPoint"))
  (for _array_element _outactors
    (Utilities|FlowControl|Sequence
      (:then_0
        (if (Actor|ActorHasTag _array_element "NPCEntrance")
          (Variables|Default|SetNPCEntranceRef _array_element)))
      (:then_1
        (if (Actor|ActorHasTag _array_element "CustomerRequestLocation")
          (Variables|Default|SetCounterLocationRef _array_element)))
      (:then_2
        (if (Actor|ActorHasTag _array_element "WorkbenchLocation")
          (Variables|Default|SetWorkbenchLocationRef _array_element)))
      (:then_3
        (Utilities|Time|SetTimerbyEvent (delegate Custom|SpawnNewCustomer) (Math|Random|RandomFloatinRange 5.0 15.0) true))
      (:then_4
        (Variables|/Script/Engine.PlayerController|SetbShowMouseCursor (Game|GetPlayerController 0) true)))))

(event EventTick
  (params (DeltaSeconds :type Float%20%28single-precision%29)))

(fn ConstructionScript)