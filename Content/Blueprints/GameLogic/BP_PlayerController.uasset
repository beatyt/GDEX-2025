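; Player controller for a furniture-buying game, handling money, item placement, and the carousel, chat log and pause menu widgets.
; InitiatePlacement spawns a preview with a dynamic outline material, which Tick moves along Floor-tagged cursor hits, tinting green or red via box trace and smoothly interpolating 45-degree rotations.
; Placing deducts cost and notifies BP_PlayerCharacter of order fulfilment.
; A looping timer pays periodic interest.
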(event Custom|InitiatePlacement
  (params (SelectedItem :type F%20Furniture%20Data%20Structure))
  (bind (_furniturename _furniturecost _furnituremesh _furnitureblueprint) (Utilities|Struct|BreakF_FurnitureData SelectedItem))
  (bind _returnvalue (Transformation|GetActorTransform))
  (bind (_location _rotation _scale) (Math|Transform|BreakTransform _returnvalue))
  (if (>= (Variables|Default|GetMoney) _furniturecost)
    (Variables|Default|SetSelected%20Item SelectedItem)
    ;[0.15 0.15 0.15 0.5 36] Placeholder
    (bind _returnvalue_2 (Game|SpawnActorfromClass _furnitureblueprint (Math|Transform|MakeTransform _location (Math|Rotator|MakeRotator 0.0 0.0 (.Yaw (Math|Rotator|BreakRotator _rotation))) _scale) "Undefined" "MultiplyWithRoot" 0 0))
    (Collision|SetCollisionResponsetoChannel (Variables|/Game/Blueprints/Furniture/BP_FurnitureBase.BP_FurnitureBase_C|GetBox _returnvalue_2) "ECC_Pawn" "ECR_Ignore")
    (bind _output_get (Variables|Default|SetCurrentPlacementActor _returnvalue_2))
    (Variables|Default|SetDesiredRotation (Transformation|GetWorldRotation (Variables|/Game/Blueprints/Furniture/BP_FurnitureBase.BP_FurnitureBase_C|GetFurnitureMesh _output_get)))
    (Variables|Default|SetIsPlacing true)
    (bind _returnvalue_3 (Rendering|Material|CreateDynamicMaterialInstance (Variables|/Game/Blueprints/Furniture/BP_FurnitureBase.BP_FurnitureBase_C|GetFurnitureMesh (Variables|Default|GetCurrentPlacementActor)) 0 "/Game/Blueprints/M_PlacementOutline.M_PlacementOutline" "None" :!class /Script/Engine.PrimitiveComponent)) ; need to make a material here
    (bind _output_get_2 (Variables|Default|SetPlacementMaterialInstance _returnvalue_3))
    (Rendering|Material|SetMaterial (Variables|/Game/Blueprints/Furniture/BP_FurnitureBase.BP_FurnitureBase_C|GetFurnitureMesh (Variables|Default|GetCurrentPlacementActor)) 0 _output_get_2)
    (else
      (Audio|PlaySound2D "/Game/Sounds/denied.denied" 1.0 1.0 0.0 0 0))))

(event Custom|RotatePlacement
  (Variables|Default|SetDesiredRotation (Math|Rotator|CombineRotators (Transformation|GetWorldRotation (Variables|/Game/Blueprints/Furniture/BP_FurnitureBase.BP_FurnitureBase_C|GetFurnitureMesh (Variables|Default|GetCurrentPlacementActor))) (Math|Rotator|MakeRotator 0.0 0.0 45.0))))

(event Custom|Timed%20Interest%20Payments
  ;[0.15 0.15 0.15 0.5 36] Begin
  (CallFunction|AwardMonies 5.0 false))

(event Input|EnhancedActionEvents|EnhancedInputActionIA_RotateItem
  (params (ActionValue :type Boolean) (ElapsedSeconds :type Float%20%28double-precision%29) (TriggeredSeconds :type Float%20%28double-precision%29) (InputAction :type Input%20Action%20Object%20Reference :default "/Game/Blueprints/GameLogic/Controls/IA_RotateItem.IA_RotateItem"))
  (CallFunction|RotatePlacement))

(event Input|EnhancedActionEvents|EnhancedInputActionIA_PlaceItem
  (params (ActionValue :type Boolean) (ElapsedSeconds :type Float%20%28double-precision%29) (TriggeredSeconds :type Float%20%28double-precision%29) (InputAction :type Input%20Action%20Object%20Reference :default "/Game/Blueprints/GameLogic/Controls/IA_PlaceItem.IA_PlaceItem"))
  (bind _selected_item (Variables|Default|GetSelected%20Item))
  (bind _furniturecost (Utilities|Struct|BreakF_FurnitureData _selected_item))
  ;[0.15 0.15 0.15 0.5 36] Mouse Click
  (if (Variables|Default|GetIsPlacing)
    (if (Variables|Default|GetIsValidPlacement)
      (if (>= (Variables|Default|GetMoney) _furniturecost)
        (bind _output_get (Variables|Default|SetMoney (- (Variables|Default|GetMoney) _furniturecost)))
        (Audio|Components|Audio|Play (Variables|Default|GetAudio) 0.0)
        (Rendering|Material|SetMaterial (Variables|/Game/Blueprints/Furniture/BP_FurnitureBase.BP_FurnitureBase_C|GetFurnitureMesh (Variables|Default|GetCurrentPlacementActor)) 0 (Rendering|Material|GetMaterial (Variables|/Game/Blueprints/Furniture/BP_FurnitureBase.BP_FurnitureBase_C|GetFurnitureMesh (Variables|Default|GetCurrentPlacementActor)) 0))
        (Utilities|FlowControl|Sequence
          (:then_0
            (Utilities|Array|Add (Variables|/Script/Engine.Actor|GetTags (Variables|Default|GetCurrentPlacementActor)) "Purchase")
            (Variables|/Script/Engine.Actor|SetTags (Variables|Default|GetCurrentPlacementActor) (Variables|/Script/Engine.Actor|GetTags (Variables|Default|GetCurrentPlacementActor)))
            (bind _outactors (Actor|GetAllActorsOfClass "/Game/Blueprints/GameLogic/BP_PlayerCharacter.BP_PlayerCharacter_C"))
            (Default|OrderFulfiled (Utilities|Array|Get(acopy) _outactors) 0 (Utilities|GetClass (Variables|Default|GetCurrentPlacementActor)) (Variables|Default|GetCurrentPlacementActor)))
          (:then_1
            (Default|OnPlace (Variables|Default|GetCurrentPlacementActor)))
          (:then_2
            (Variables|Default|SetCurrentPlacementActor 0)
            (Variables|Default|SetIsPlacing false)))
        (else
          (Development|PrintString "Not Enough Cash" true true "(R=0.000000,G=0.660000,B=1.000000,A=1.000000)" _output_get)
          (Actor|DestroyActor (Variables|Default|GetCurrentPlacementActor))
          (Variables|Default|SetIsPlacing false))))))

(event Input|EnhancedActionEvents|EnhancedInputActionIA_PauseMenu
  (params (ActionValue :type Boolean) (ElapsedSeconds :type Float%20%28double-precision%29) (TriggeredSeconds :type Float%20%28double-precision%29) (InputAction :type Input%20Action%20Object%20Reference :default "/Game/Blueprints/GameLogic/Controls/IA_PauseMenu.IA_PauseMenu"))
  (UserInterface|Viewport|AddtoViewport (Variables|Default|GetPauseMenu) 0)
  (Game|SetGamePaused true))

(event Input|EnhancedActionEvents|EnhancedInputActionIA_CancelPlacement
  (params (ActionValue :type Boolean) (ElapsedSeconds :type Float%20%28double-precision%29) (TriggeredSeconds :type Float%20%28double-precision%29) (InputAction :type Input%20Action%20Object%20Reference :default "/Game/Blueprints/GameLogic/Controls/IA_CancelPlacement.IA_CancelPlacement"))
  (Utilities|IsValid (Variables|Default|GetCurrentPlacementActor)
    (:Is%20Valid
      (Actor|DestroyActor (Variables|Default|GetCurrentPlacementActor))
      (Variables|Default|SetCurrentPlacementActor 0)
      (Variables|Default|SetIsPlacing false)
      (Variables|Default|SetDesiredRotation "0, 0, 0"))))

(event EventBeginPlay
  ;[0.15 0.15 0.15 0.5 36] Begin
  (Utilities|FlowControl|Sequence
    (:then_0
      (Input|AddMappingContext (PlayerController|LocalPlayerSubsystems|GetEnhancedInputLocalPlayerSubsystem (Game|GetPlayerController 0)) "/Game/Blueprints/GameLogic/Controls/IMC_PlayerControls.IMC_PlayerControls" 0 "(bIgnoreAllPressedKeysUntilRelease=True,bForceImmediately=False,bNotifyUserSettings=False)")
      (bind _returnvalue (UserInterface|CreateWidget "/Game/Blueprints/Widgets/WBP_FurnitureCarousel.WBP_FurnitureCarousel_C"))
      (UserInterface|Viewport|AddtoViewport _returnvalue 0)
      (bind _returnvalue_2 (UserInterface|CreateWidget "/Game/Blueprints/Widgets/WBP_ChatLog.WBP_ChatLog_C"))
      (UserInterface|Viewport|AddtoViewport _returnvalue_2 0)
      (Variables|Default|SetChatLogRef _returnvalue_2))
    (:then_1
      (Utilities|Time|SetTimerbyEvent (delegate Custom|Timed%20Interest%20Payments) 5.0 true))
    (:then_2
      (bind _returnvalue_3 (UserInterface|CreateWidget "/Game/Blueprints/Widgets/WBP_PauseMenu.WBP_PauseMenu_C"))
      (Variables|Default|SetPauseMenu _returnvalue_3))))

(event EventTick
  (params (DeltaSeconds :type Float%20%28single-precision%29))
  (bind (_locationx _locationy) (Game|Player|GetMousePosition))
  (bind _returnvalue (Game|GetPlayerController 0))
  (bind _currentplacementactor (Variables|Default|GetCurrentPlacementActor))
  (bind _currentplacementactor_2 (Variables|Default|GetCurrentPlacementActor))
  (bind _placementmaterialinstance (Variables|Default|GetPlacementMaterialInstance))
  (bind _returnvalue_2 (Actor|GetComponentbyClass _currentplacementactor_2 "/Script/Engine.BoxComponent"))
  (bind (_worldlocation _worlddirection) (Class|PlayerController|DeprojectScreenPositiontoWorld _returnvalue _locationx _locationy))
  (bind _furnituremesh (Variables|/Game/Blueprints/Furniture/BP_FurnitureBase.BP_FurnitureBase_C|GetFurnitureMesh _currentplacementactor))
  (bind _overlappingactors (Collision|GetOverlappingActors _returnvalue_2 0 :!class /Script/Engine.PrimitiveComponent))
  ;[0.15 0.15 0.15 0.5 36] Placements
  (Utilities|FlowControl|Sequence
    (:then_0
      (if (Variables|Default|GetIsPlacing)
        (bind (_outhit _returnvalue_3) (Collision|LineTraceByChannel (.Location (Pawn|GetPlayerViewPoint)) (+ _worldlocation (* _worlddirection 1e+04)) "TraceTypeQuery1" false 0 "None"))
        (if _returnvalue_3
          (if (Actor|ActorHasTag (.HitActor (Collision|BreakHitResult _outhit)) "Floor")
            (Transformation|SetActorLocation _currentplacementactor_2 (Math|Vector|MakeVector (.X (Math|Vector|BreakVector (.Location (Collision|BreakHitResult _outhit)))) (.Y (Math|Vector|BreakVector (.Location (Collision|BreakHitResult _outhit)))) (.Z (Math|Vector|BreakVector (.Location (Collision|BreakHitResult _outhit))))) false false)
            (bind _outactors (Actor|GetAllActorsOfClass "/Script/Engine.TriggerVolume"))
            (for _array_element _outactors
              (Utilities|Array|RemoveItem _overlappingactors _array_element))
            (if (<= (Utilities|Array|Length _overlappingactors) 1)
              (bind _returnvalue_4 (Actor|GetActorOfClass "/Script/Landscape.Landscape"))
              (bind (_outhit_2 _returnvalue_5) (Class|KismetSystemLibrary|BoxTraceSingleforObjects (.Location (Collision|BreakHitResult _outhit)) (.Location (Collision|BreakHitResult _outhit)) (.BoxExtent (Collision|GetActorBounds _currentplacementactor_2 true false)) "0, 0, 0" (Utilities|Array|MakeArray "ObjectTypeQuery1" "ObjectTypeQuery2") false (Utilities|Array|MakeArray (Variables|Default|GetCurrentPlacementActor) _returnvalue_4) "None" true))
              (if _returnvalue_5
                (Development|PrintString (Utilities|GetDisplayName (.HitActor (Collision|BreakHitResult _outhit_2))))
                (Rendering|Material|SetVectorParameterValue _placementmaterialinstance "Color" "(R=1.000000,G=0.000000,B=0.000000,A=1.000000)" :!class /Script/Engine.MaterialInstanceDynamic)
                (Variables|Default|SetIsValidPlacement false)
                (else
                  (Rendering|Material|SetVectorParameterValue _placementmaterialinstance "Color" "(R=0.000000,G=1.000000,B=0.000000,A=1.000000)" :!class /Script/Engine.MaterialInstanceDynamic)
                  (Variables|Default|SetIsValidPlacement true))))))))
    (:then_1
      (Utilities|IsValid (Variables|Default|GetCurrentPlacementActor)
        (:Is%20Valid
          (Transformation|SetWorldRotation _furnituremesh (Math|Interpolation|RInterpTo (Transformation|GetWorldRotation _furnituremesh) (Variables|Default|GetDesiredRotation) DeltaSeconds 1e+01) false false))))))

(fn ConstructionScript)

(fn AwardMonies
  (params (Amount :type Float%20%28double-precision%29) (PlaySfx? :type Boolean))
  (Variables|Default|SetMoney (+ (Variables|Default|GetMoney) Amount))
  (if PlaySfx?
    (Audio|Components|Audio|Play (Variables|Default|GetAudio) 0.0)))

(fn DeductMonies
  (params (Amount :type Float%20%28double-precision%29))
  (CallFunction|AwardMonies (* -1.0 Amount) true))

(fn UpdateChatLog
  (bind _chathistory (Variables|Default|GetChatHistory))
  (bind _chatlogref (Variables|Default|GetChatLogRef))
  (bind _chatscroll (Variables|/Game/Blueprints/Widgets/WBP_ChatLog.WBP_ChatLog_C|GetChatScroll _chatlogref))
  (Widget|Panel|ClearChildren _chatscroll)
  (Utilities|Array|Reverse _chathistory)
  (for _array_element _chathistory
    (bind _returnvalue (UserInterface|CreateWidget "/Game/Blueprints/Widgets/WBP_ChatLogItem.WBP_ChatLogItem_C"))
    (Rendering|Components|TextRender|SetText (Variables|/Game/Blueprints/Widgets/WBP_ChatLogItem.WBP_ChatLogItem_C|GetChatItem _returnvalue) (Utilities|Text|ToText(String) _array_element))
    (Widget|Panel|AddChild _chatscroll _returnvalue))
  (Class|ScrollBox|ScrolltoEnd _chatscroll))