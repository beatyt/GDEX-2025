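; Corrupted customer AI that steals items implementing BPI_Stealable.
; On BeginPlay, a random roll checked against its previous action selects either theft or walking to the Shop trigger volume.
; Theft picks a random stealable, retrying if tagged Stolen, then moves nearby, attaches it to the hand, tags it and ends the interaction.
; BeginInteraction forwards to the shopkeeper, and Polymorph clears the Stolen tag from the initially chosen target.
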(event Custom|Find%20Something%20To%20Steal
  (params (Target :type Actor%20Object%20Reference))
  ;[0.15 0.15 0.15 0.5] Steal
  (bind _asbpi_stealable (Utilities|Casting|CastToBPI_Stealable Target))
  (if (Actor|ActorHasTag Target "Stolen")
    (Utilities|FlowControl|Delay 2.0)
    (bind _desiredactor (CallFunction|FindStealables))
    (CallFunction|FindSomethingtoSteal _desiredactor)
    (else
      (CallFunction|Steal _asbpi_stealable))))

(event EventBeginPlay
  ;[0.15 0.15 0.15 0.5] Steal
  (|CallParentFunction)
  (bind _output_get (Variables|Default|SetCurrent%20Action (Math|Random|RandomBool)))
  (if (Math|Boolean|NANDBoolean _output_get (Variables|Default|GetPreviousAction))
    (Variables|Default|SetPreviousAction _output_get)
    (bind _desiredactor (CallFunction|FindStealables))
    (Variables|Default|SetDesired%20Actor _desiredactor)
    (CallFunction|FindSomethingtoSteal _desiredactor)
    (else
      (Variables|Default|SetPreviousAction _output_get)
      (bind _outactors (Actor|GetAllActorsOfClasswithTag "/Script/Engine.TriggerVolume" "Shop"))
      (AI|AIMoveTo self "0, 0, 0" (Utilities|Array|Get(acopy) _outactors) 5.0 false))))

(event Collision|EventActorBeginOverlap
  (params (OtherActor :type Actor%20Object%20Reference)))

(event EventPolymorph
  (bind _desired_actor (Variables|Default|GetDesired%20Actor))
  (|CallParentFunction)
  (Utilities|IsValid _desired_actor
    (:Is%20Valid
      (Utilities|Array|RemoveItem (Variables|/Script/Engine.Actor|GetTags _desired_actor) "Stolen"))))

(event EventTick
  (params (DeltaSeconds :type Float%20%28single-precision%29)))

(event EventEndInteraction
  (params (Sender :type BPI%20Interaction%20Interface))
  ;[0.15 0.15 0.15 0.5 36] Interactions
  (|CallParentFunction Sender))

(event EventBeginInteraction
  (params (Sender :type BPI%20Interaction%20Interface) (InteractionMetadata :type S%20Interaction%20Metadata%20Structure))
  ;[0.15 0.15 0.15 0.5 36] Interactions
  (bind _returnvalue (Actor|GetActorOfClass "/Game/Blueprints/BP_Shopkeep.BP_Shopkeep_C"))
  (Default|BeginInteraction _returnvalue self))

(event EventUpdate
  (params (Sender :type BPI%20Interaction%20Interface) (InteractionMetadata :type S%20Interaction%20Metadata%20Structure))
  ;[0.15 0.15 0.15 0.5 36] Interactions
)

(event EventBeginPurchase
  (params (Purchase :type S%20Purchase%20Structure) (RequestingCustomer :type BPI%20Interaction%20Interface))
  ;[0.15 0.15 0.15 0.5 36] Interactions
)

(event EventEndPurchase
  (params (Purchase :type S%20Purchase%20Structure) (ShouldPay? :type Boolean))
  ;[0.15 0.15 0.15 0.5 36] Interactions
)

(event EventSteal
  (params (Target :type BPI%20Stealable%20Interface))
  ;[0.15 0.15 0.15 0.5 36] Interactions
  (bind _asactor (Utilities|Casting|CastToActor Target))
  (bind _randomlocation (Class|NavigationSystemV1|GetRandomLocationinNavigableRadius (Transformation|GetActorLocation _asactor) 125.0 0 0))
  (AI|AIMoveTo self _randomlocation 0 1e+02 true
    (:OnSuccess
      (Collision|SetActorEnableCollision _asactor false)
      (Transformation|AttachActorToActor _asactor self "hand" "SnapToTarget" "SnapToTarget" "SnapToTarget" true)
      (Utilities|Array|Add (Variables|/Script/Engine.Actor|GetTags _asactor) "Stolen")
      (CallFunction|EndInteraction))
    (:OnFail
      (Utilities|FlowControl|Delay 2.0)
      (CallFunction|Steal Target))))

(fn ConstructionScript)

(fn FindStealables
  (bind _outactors (Actor|GetAllActorswithInterface "/Game/Blueprints/BPI_Stealable.BPI_Stealable_C"))
  (return (.OutItem (Utilities|Array|Random _outactors))))