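; Base customer character for a furniture shop game that requests a random data-table item, chats, pays and leaves.
; Interaction starts a timer-driven patience bar facing the camera; running out ends the visit unpaid.
; Updates either place an order with the player or send the customer via AI MoveTo to collect "Purchase"-tagged furniture, pay a hardcoded amount and head for the exit.
; Polymorph replaces the customer with a pig.
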(event Custom|SetRequestedItem
  (params (ItemToRequest :type F%20Furniture%20Data%20Structure))
  (Variables|Default|SetRequestedFurniture ItemToRequest))

(event Custom|SaySomethingFunny
  ;[0.15 0.15 0.15 0.5] Dialog
  (bind _aswbp_chat_bubble (Utilities|Casting|CastToWBP_ChatBubble (UserInterface|GetUserWidgetObject (Variables|Default|GetChatBubbleComponent))))
  (bind _output_get (Variables|Default|SetLastFunnySaid (.OutItem (Utilities|Array|Random (Variables|Default|GetFunnyComments)))))
  (Rendering|Components|TextRender|SetText (Variables|/Game/Blueprints/Widgets/WBP_ChatBubble.WBP_ChatBubble_C|GetChat _aswbp_chat_bubble) _output_get)
  (Default|PlayAnim _aswbp_chat_bubble)
  (Widget|SetVisibility (Variables|/Game/Blueprints/Widgets/WBP_ChatBubble.WBP_ChatBubble_C|GetChat _aswbp_chat_bubble) "Visible")
  (Utilities|Time|SetTimerbyEvent (delegate Custom|HideChatBubble) 1e+01)
  (bind _asbp_player_controller (Utilities|Casting|CastToBP_PlayerController (Game|GetPlayerController 0)))
  (Utilities|Array|Add (Variables|/Game/Blueprints/GameLogic/BP_PlayerController.BP_PlayerController_C|GetChatHistory _asbp_player_controller) (Utilities|String|ToString(Text) _output_get))
  (Default|UpdateChatLog _asbp_player_controller))

(event Custom|CustomEvent
  ;[0.15 0.15 0.15 0.5] Dialog
  (Widget|SetVisibility (Variables|/Game/Blueprints/Widgets/WBP_ChatBubble.WBP_ChatBubble_C|GetChat (stale Custom|Give%20Thanks _aswbp_chat_bubble)) "Hidden"))

(event Custom|Polymorph
  (Variables|/Script/Engine.CharacterMovementComponent|SetMaxWalkSpeed (Variables|Character|GetCharacterMovement) 0.0)
  (Actor|SetLifeSpan 0.3)
  (Utilities|FlowControl|Delay 0.3)
  (Game|SpawnActorfromClass "/Game/Blueprints/Customers/BP_Pig.BP_Pig_C" (Transformation|GetActorTransform) "Undefined" "MultiplyWithRoot" 0 false 0))

(event Custom|TakeOrderObject
  (params (Object :type BP%20Furniture%20Base%20Object%20Reference))
  (Development|PrintString "Taking order object ")
  (bind _randomlocation (Class|NavigationSystemV1|GetRandomLocationinNavigableRadius (Transformation|GetActorLocation Object) 25.0 0 0))
  (bind _movementresult (AI|AIMoveTo self _randomlocation 0 1.5e+02 true)
    (:OnSuccess
      (Collision|SetActorEnableCollision Object false)
      (Transformation|AttachActorToActor Object self "hand" "SnapToTarget" "SnapToTarget" "SnapToTarget" true)
      (CallFunction|EndPurchase :ShouldPay? true))
    (:OnFail
      (Development|PrintString (Utilities|String|EnumtoString _movementresult))
      (Utilities|FlowControl|Delay 2.0)
      (CallFunction|TakeOrderObject Object))))

(event Custom|Give%20Thanks
  ;[0.15 0.15 0.15 0.5] Dialog
  (bind _aswbp_chat_bubble (Utilities|Casting|CastToWBP_ChatBubble (UserInterface|GetUserWidgetObject (Variables|Default|GetChatBubbleComponent))))
  (Rendering|Components|TextRender|SetText (Variables|/Game/Blueprints/Widgets/WBP_ChatBubble.WBP_ChatBubble_C|GetChat _aswbp_chat_bubble) "Thanks")
  (Default|PlayAnim _aswbp_chat_bubble)
  (Widget|SetVisibility (Variables|/Game/Blueprints/Widgets/WBP_ChatBubble.WBP_ChatBubble_C|GetChat _aswbp_chat_bubble) "Visible")
  (Utilities|Time|SetTimerbyEvent (delegate Custom|CustomEvent) 3.0))

(event Custom|HideChatBubble
  ;[0.15 0.15 0.15 0.5] Dialog
  (Widget|SetVisibility (Variables|/Game/Blueprints/Widgets/WBP_ChatBubble.WBP_ChatBubble_C|GetChat (stale Custom|SaySomethingFunny _aswbp_chat_bubble)) "Hidden"))

(event Custom|Countdown
  (Variables|Default|SetWaitProgress (- (Variables|Default|GetWaitProgress) 0.02))
  (bind _aswbp_progress (Utilities|Casting|CastToWBP_Progress (UserInterface|GetWidget (Variables|Default|GetProgress))))
  (Default|UpdateProgress _aswbp_progress (Variables|Default|GetWaitProgress))
  (if (<= (Variables|Default|GetWaitProgress) 0.0)
    (Utilities|FlowControl|DoOnce false
      (:Completed
        (Widget|SetVisibility (UserInterface|GetWidget (Variables|Default|GetProgress)) "Hidden")
        (if (not (Variables|Default|GetPurchaseComplete?))
          (CallFunction|EndPurchase))))))

(event Custom|StartCountdown
  (bind _progress (Variables|Default|GetProgress))
  (bind _returnvalue (UserInterface|GetWidget _progress))
  (bind _aswbp_progress (Utilities|Casting|CastToWBP_Progress _returnvalue))
  (Variables|Default|SetWaitProgress 1.0)
  (Widget|SetVisibility _returnvalue "Visible") ; This would not show reliably...
  (Utilities|Time|SetTimerbyEvent (delegate Custom|Countdown) 0.5 true))

(event EventBeginPlay
  (Utilities|FlowControl|Sequence
    (:then_0
      (CallFunction|SaySomethingFunny)
      (bind _outrownames (DataTable|GetDataTableRowNames "/Game/Blueprints/Data/DT_FurnitureData.DT_FurnitureData"))
      (bind _returnvalue (Utilities|GetDataTableRow "/Game/Blueprints/Data/DT_FurnitureData.DT_FurnitureData" (.OutItem (Utilities|Array|Random _outrownames)))
        (:then
          (Variables|Default|SetRequestedFurniture _returnvalue))))))

(event Collision|EventActorBeginOverlap
  (params (OtherActor :type Actor%20Object%20Reference)))

(event EventTick
  (params (DeltaSeconds :type Float%20%28single-precision%29))
  (Transformation|SetWorldRotation (Variables|Default|GetProgress) (Math|Rotator|FindLookatRotation (Transformation|GetWorldLocation (Variables|Default|GetProgress)) (Transformation|GetWorldLocation (Variables|/Script/Engine.PlayerCameraManager|GetTransformComponent (Game|GetPlayerCameraManager 0)))) false false))

(event EventEndInteraction
  (params (Sender :type BPI%20Interaction%20Interface))
  (Development|PrintString (Utilities|String|Append (Utilities|GetDisplayName self) " is leaving"))
  (bind _outactors (Actor|GetAllActorsOfClasswithTag "/Script/Engine.TriggerVolume" "Exit"))
  (AI|AIMoveTo self "0, 0, 0" (Utilities|Array|Get(acopy) _outactors) 25.0 true
    (:OnFail
      (Development|PrintString "Movement failed")
      (Utilities|FlowControl|Delay 5.0)
      (CallFunction|EndInteraction))))

(event EventBeginInteraction
  (params (Sender :type BPI%20Interaction%20Interface) (InteractionMetadata :type S%20Interaction%20Metadata%20Structure))
  (Utilities|FlowControl|DoOnce false
    (:Completed
      (CallFunction|StartCountdown))))

(event EventBeginPurchase
  (params (Purchase :type S%20Purchase%20Structure) (RequestingCustomer :type BPI%20Interaction%20Interface))
  (Utilities|FlowControl|DoOnce false
    (:Completed
      (bind _outactors (Actor|GetAllActorsOfClass "/Game/Blueprints/GameLogic/BP_PlayerCharacter.BP_PlayerCharacter_C"))
      (bind _asbp_player_character (Utilities|Casting|CastToBP_PlayerCharacter (Utilities|Array|Get(acopy) _outactors)))
      (Default|OrderPlaced _asbp_player_character (.ActorRef (Utilities|Struct|BreakS_Purchase Purchase)) self))))

(event EventEndPurchase
  (params (Purchase :type S%20Purchase%20Structure) (ShouldPay? :type Boolean))
  (Utilities|FlowControl|DoOnce false
    (:Completed
      (Variables|Default|SetWaitProgress 0.0) ; Would be better as its own event
      (bind _outactors (Actor|GetAllActorsOfClass "/Game/Blueprints/GameLogic/BP_PlayerCharacter.BP_PlayerCharacter_C"))
      (bind _asbp_player_character (Utilities|Casting|CastToBP_PlayerCharacter (Utilities|Array|Get(acopy) _outactors)))
      (if ShouldPay?
        (CallFunction|PayforPurchase (Utilities|Struct|MakeF_FurnitureData "" 0.0 0 0 1e+02))
        (CallFunction|GiveThanks)
        (Utilities|FlowControl|Delay 0.3) ; Idk man
        (CallFunction|EndInteraction self) ; Do not end interaction here, it overwrites movement to get order
        (else
          (Default|EndInteraction _asbp_player_character self)
          (CallFunction|EndInteraction))))))

(event EventUpdate
  (params (Sender :type BPI%20Interaction%20Interface) (InteractionMetadata :type S%20Interaction%20Metadata%20Structure))
  (bind _orderisready_ (Utilities|Struct|BreakS_InteractionMetadata InteractionMetadata))
  ;[0.15 0.15 0.15 0.5 72] Receive
  (Variables|Default|SetPurchaseComplete? _orderisready_)
  (if _orderisready_
    (bind _object (CallFunction|FindReadyOrders))
    (CallFunction|TakeOrderObject _object)
    (else
      (Default|ReceiveUpdate Sender self (Utilities|Struct|MakeS_InteractionMetadata true (Variables|Default|GetRequestedFurniture)))
      (CallFunction|BeginPurchase (Utilities|Struct|MakeS_Purchase 0.0 "None" 0) self) ; Hardcoded Purchasing
    )))

(fn ConstructionScript)

(fn FindReadyOrders
  (bind _outactors (Actor|GetAllActorswithTag "Purchase"))
  (bind _asbp_furniture_base (Utilities|Casting|CastToBP_FurnitureBase (Utilities|Array|Get(acopy) _outactors)))
  (return _asbp_furniture_base))

(fn PayforPurchase
  (params (RequestedFurniture :type F%20Furniture%20Data%20Structure))
  (bind _asbp_player_controller (Utilities|Casting|CastToBP_PlayerController (Game|GetPlayerController 0)))
  (Default|AwardMonies _asbp_player_controller (.FurnitureProfit (Utilities|Struct|BreakF_FurnitureData RequestedFurniture)) true)
  ;[0.15 0.15 0.15 0.5] Not great since it removes it from everything but the other code looks for the first one
  (bind _outactors (Actor|GetAllActorswithTag "Purchase"))
  (for _array_element _outactors
    (Utilities|Array|RemoveItem (Variables|/Script/Engine.Actor|GetTags _array_element) "Purchase")))