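; BP_Patron is a customer that walks to a Shop-tagged trigger volume on spawn to order furniture.
; On interaction it plays Speak and messages the shopkeep through BPI_Interaction.
; Updates either send the requested furniture to the sender and begin a hardcoded purchase, or collect the ready order and end the purchase.
; Interaction and purchase events extend parent logic; payment and money-award nodes here are unconnected.
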(event EventBeginPlay
  (|CallParentFunction)
  (bind _outactors (Actor|GetAllActorsOfClasswithTag "/Script/Engine.TriggerVolume" "Shop"))
  (AI|AIMoveTo self "0, 0, 0" (Utilities|Array|Get(acopy) _outactors) 5.0 false))

(event Collision|EventActorBeginOverlap
  (params (OtherActor :type Actor%20Object%20Reference)))

(event EventTick
  (params (DeltaSeconds :type Float%20%28single-precision%29)))

(event EventEndInteraction
  (params (Sender :type BPI%20Interaction%20Interface))
  ;[0.15 0.15 0.15 0.5 36] Interactions
  (|CallParentFunction Sender))

(event EventBeginInteraction
  (params (Sender :type BPI%20Interaction%20Interface) (InteractionMetadata :type S%20Interaction%20Metadata%20Structure))
  ;[0.15 0.15 0.15 0.5 36] Interactions
  (|CallParentFunction Sender InteractionMetadata)
  (Audio|Components|Audio|Play (Variables|Default|GetSpeak) 0.0)
  (bind _returnvalue (Actor|GetActorOfClass "/Game/Blueprints/BP_Shopkeep.BP_Shopkeep_C"))
  (if (Utilities|DoesObjectImplementInterface _returnvalue "/Game/Blueprints/BPI_Interaction.BPI_Interaction_C")
    (Class|BPIInteraction|BeginInteraction(Message) _returnvalue self)))

(event EventUpdate
  (params (Sender :type BPI%20Interaction%20Interface) (InteractionMetadata :type S%20Interaction%20Metadata%20Structure))
  ;[0.15 0.15 0.15 0.5 36] Interactions
  (if (.OrderIsReady? (Utilities|Struct|BreakS_InteractionMetadata InteractionMetadata))
    (bind _object (CallFunction|FindReadyOrders))
    (CallFunction|TakeOrderObject _object)
    (CallFunction|EndPurchase)
    (else
      (Default|ReceiveUpdate Sender self (Utilities|Struct|MakeS_InteractionMetadata true (Variables|Default|GetRequestedFurniture)))
      (CallFunction|BeginPurchase (Utilities|Struct|MakeS_Purchase 0.0 "None" 0) self) ; Hardcoded Purchasing
    )))

(event EventBeginPurchase
  (params (Purchase :type S%20Purchase%20Structure) (RequestingCustomer :type BPI%20Interaction%20Interface))
  ;[0.15 0.15 0.15 0.5] Purchases
  (|CallParentFunction Purchase RequestingCustomer))

(event EventEndPurchase
  (params (Purchase :type S%20Purchase%20Structure))
  ;[0.15 0.15 0.15 0.5] Purchases
  (|CallParentFunction Purchase))

(fn ConstructionScript)