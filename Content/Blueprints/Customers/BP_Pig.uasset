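; BP_Pig is an AI-moved pig that either wanders or heads for the exit, depending on IsWanderer.
; Wanderers loop through AIMoveTo to random navigable points nearby, pausing a random interval after each success or failure.
; Non-wanderers oink shortly after BeginPlay and move to the first TriggerVolume tagged Exit.
; BeginTheft plays an oink at the pig's location, while EndTheft is empty.
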(event Custom|Wander
  (bind _returnvalue (Math|Random|RandomFloatinRange 5.0 15.0))
  (bind _randomlocation (Class|NavigationSystemV1|GetRandomLocationinNavigableRadius (Transformation|GetActorLocation) 512.0 0 0))
  (AI|AIMoveTo self _randomlocation 0 5.0 false
    (:OnSuccess
      (Utilities|FlowControl|Delay _returnvalue)
      (CallFunction|Wander))
    (:OnFail
      (Utilities|FlowControl|Delay _returnvalue)
      (CallFunction|Wander))))

(event EventBeginPlay
  (if (Variables|Default|GetIsWanderer?)
    (CallFunction|Wander)
    (else
      (Utilities|FlowControl|Delay 0.1)
      (Audio|Components|Audio|Play (Variables|Default|Getoink) 0.0)
      (bind _outactors (Actor|GetAllActorsOfClasswithTag "/Script/Engine.TriggerVolume" "Exit"))
      (AI|AIMoveTo self "0, 0, 0" (Utilities|Array|Get(acopy) _outactors) 5.0 false))))

(event Collision|EventActorBeginOverlap
  (params (OtherActor :type Actor%20Object%20Reference)))

(event EventTick
  (params (DeltaSeconds :type Float%20%28single-precision%29)))

(event EventBeginTheft
  (params (Stealer :type BPI%20Criminal%20Interface))
  (Audio|PlaySoundatLocation "/Game/Sounds/oink.oink" (Transformation|GetActorLocation) "0, 0, 0" 1.0 1.0 0.0 0 0 0 0))

(event EventEndTheft
  (params (Stealer :type BPI%20Criminal%20Interface)))

(fn ConstructionScript)