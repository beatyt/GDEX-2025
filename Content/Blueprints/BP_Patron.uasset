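; BP_Patron is a customer pawn that walks to the shop, requests furniture and pays the player on purchase.
; It finds the tagged Shop and Exit trigger volumes and moves between them with AI MoveTo.
; Interaction plays Speak and messages BP_Shopkeep through BPI_Interaction.
; Update returns the requested furniture to the sender, then immediately completes the purchase, awarding its profit through BP_PlayerController and sending the patron out.
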(event EventBeginPlay
  (|CallParentFunction)
  (bind _outactors (Actor|GetAllActorsOfClasswithTag "/Script/Engine.TriggerVolume" "Shop"))
  (AI|AIMoveTo self "0, 0, 0" (Utilities|Array|Get(acopy) _outactors) 5.0 false))

(event Collision|EventActorBeginOverlap
  (params (OtherActor :type Actor%20Object%20Reference)))

(event EventTick
  (params (DeltaSeconds :type Float%20%28single-precision%29)))

(event EventEndInteraction
  (params (Sender :type BPI%20Interaction%20Interface))
  ;[0.15 0.15 0.15 0.5 36] Interactions
  (bind _outactors (Actor|GetAllActorsOfClasswithTag "/Script/Engine.TriggerVolume" "Exit"))
  (AI|AIMoveTo self "0, 0, 0" (Utilities|Array|Get(acopy) _outactors) 5.0 false))

(event EventBeginInteraction
  (params (Sender :type BPI%20Interaction%20Interface) (InteractionMetadata :type S%20Interaction%20Metadata%20Structure))
  ;[0.15 0.15 0.15 0.5 36] Interactions
  (Audio|Components|Audio|Play (Variables|Default|GetSpeak) 0.0)
  (bind _returnvalue (Actor|GetActorOfClass "/Game/Blueprints/BP_Shopkeep.BP_Shopkeep_C"))
  (if (Utilities|DoesObjectImplementInterface _returnvalue "/Game/Blueprints/BPI_Interaction.BPI_Interaction_C")
    (Class|BPIInteraction|BeginInteraction(Message) _returnvalue self)))

(event EventUpdate
  (params (Sender :type BPI%20Interaction%20Interface) (InteractionMetadata :type S%20Interaction%20Metadata%20Structure))
  ;[0.15 0.15 0.15 0.5 36] Interactions
  (Default|ReceiveUpdate Sender self (Utilities|Struct|MakeS_InteractionMetadata true (Variables|Default|GetRequestedFurniture) false))
  (CallFunction|BeginPurchase))

(event EventBeginPurchase
  (params (Purchase :type S%20Purchase%20Structure))
  (CallFunction|EndPurchase))

(event EventEndPurchase
  (params (Purchase :type S%20Purchase%20Structure))
  (bind _asbp_player_controller (Utilities|Casting|CastToBP_PlayerController (Game|GetPlayerController 0)))
  (Default|AwardMonies _asbp_player_controller (.furnitureprofit (Variables|Default|GetRequestedFurniture)))
  (CallFunction|EndInteraction))

(fn ConstructionScript)