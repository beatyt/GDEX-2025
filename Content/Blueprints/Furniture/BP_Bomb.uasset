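; Placeable bomb furniture that polymorphs nearby customers when it explodes.
; Placing it starts the fuse sound and a short delay, then GoBoom fires the burst effect and explosion sound, hides the mesh and sets a lifespan for cleanup.
; GoBoom finds targets by distance-checking every BP_CustomerBase actor in the level; the Sphere overlap query for BP_Corrupted is left unused.
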(event Custom|Go%20Boom
  (Components|Activation|Activate (Variables|Default|GetCloudBurst) false)
  (Audio|Components|Audio|Play (Variables|Default|Getkaboom) 0.0)
  (Development|SetHiddeninGame (Variables|Default|GetFurnitureMesh) true true)
  (Actor|SetLifeSpan 5.0)
  (bind _outactors (Actor|GetAllActorsOfClass "/Game/Blueprints/Customers/BP_CustomerBase.BP_CustomerBase_C"))
  (for _array_element _outactors
    (if (<= (Math|Vector|VectorLength (- (Transformation|GetActorLocation) (Transformation|GetActorLocation _array_element))) 512.0)
      (bind _asbp_customer_base (Utilities|Casting|CastToBP_CustomerBase _array_element))
      (Default|Polymorph _asbp_customer_base))))

(event EventBeginPlay)

(event Collision|EventActorBeginOverlap
  (params (OtherActor :type Actor%20Object%20Reference)))

(event EventTick
  (params (DeltaSeconds :type Float%20%28single-precision%29)))

(event EventOnPlace
  (Audio|Components|Audio|Play (Variables|Default|Getfuse) 0.0)
  (Utilities|FlowControl|Delay 5.0)
  (CallFunction|GoBoom))

(fn ConstructionScript)